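; Enemy AI controller that runs the Enemy_BT behavior tree on possess and feeds perception results into its Blackboard.
; Sensing an actor tagged Player cancels the lost-sight timer and sets HasLineOfSight and TargetActor.
; Any other perception update starts a one-shot grace timer, which clears both keys when it expires.
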(event OnTargetPerceptionUpdated(AIPerception)
  (params (Actor :type Actor%20Object%20Reference) (Stimulus :type AI%20Stimulus%20Structure))
  (Variables|Default|SetSensedPawn Actor)
  (if (and (Actor|ActorHasTag Actor "Player") (Utilities|Struct|BreakAIStimulus Stimulus))
    (Utilities|Time|ClearandInvalidateTimerbyHandle (Variables|Default|GetLostSightHandle))
    (CallFunction|UpdateSight true)
    (CallFunction|UpdateTargetActor (Variables|Default|GetSensedPawn))
    (else
      (bind _returnvalue (Utilities|Time|SetTimerbyEvent (delegate Custom|NoPlayerFound) (Variables|Default|GetLostSightTimer)))
      (Variables|Default|SetLostSightHandle _returnvalue))))

(event Custom|NoPlayerFound
  (CallFunction|UpdateSight false)
  (CallFunction|UpdateTargetActor))

(event EventBeginPlay)

(event EventTick
  (params (DeltaSeconds :type Float%20%28single-precision%29)))

(event EventPossess
  (params (PossessedPawn :type Pawn%20Object%20Reference))
  (AI|RunBehaviorTree "/Game/blueprints/AI/Enemy_BT.Enemy_BT"))

(fn ConstructionScript)

(fn UpdateSight
  (params (SightStatus :type Boolean))
  (AI|Components|Blackboard|SetValueasBool (Variables|Default|GetBlackboard) (Variables|Default|GetHasLineOfSight) SightStatus))

(fn UpdateTargetActor
  (params (TargetActor :type Actor%20Object%20Reference))
  (AI|Components|Blackboard|SetValueasObject (Variables|Default|GetBlackboard) (Variables|Default|GetTargetActor) TargetActor))